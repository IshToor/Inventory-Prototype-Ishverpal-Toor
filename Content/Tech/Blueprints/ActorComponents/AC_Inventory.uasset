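; Actor component that manages a fixed-slot player inventory with stacking, dropping and sorting.
; Init sizes the slot array, binds events and initializes the inventory widget.
; Pickups fill stacks or empty slots, re-running pickup for overflow and updating the widget, while drops respawn items with their stats at random reachable points nearby.
; Sorting strips empty slots, bubble-sorts by quantity or recursively groups by class, then restores empty slots.
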(event Custom|SortItemsByQuantity
  ;[1 1 1] Sort Items By Quantity - Filters out empty slots before sorting inventory from largest to smallest
  (bind _filteredoutemptyslots (CallFunction|FilterEmptySlots))
  (CallFunction|SortbyQuantity _filteredoutemptyslots))

(event Custom|ItemPickUp
  (params (ItemClass :type BP%20Base%20Item%20Class%20Reference) (ItemRef :type BP%20Base%20Item%20Object%20Reference))
  ;[1 1 1] Item Pick Up - Attempts to add the item to the inventory.
  (bind (_isitemadded _slotindex _slotinfo) (CallFunction|AddItem ItemClass ItemRef))
  (if _isitemadded
    (Development|PrintString "Item was added")
    (Default|CallOnItemAdded (Variables|/Game/Tech/Blueprints/UI/W_MasterHUD.W_MasterHUD_C|GetW_MainInventory (Variables|Default|GetInventoryMenu)) _slotindex _slotinfo)
    (if (!= ItemRef 0)
      (Actor|DestroyActor ItemRef))
    (else
      (Development|PrintString "Item wasn't added"))))

(event Custom|SortItemsByItemClass
  ;[1 1 1] Sort Items By Item Class - Filters out empty slots, finds all current item classes to loop through and sort by
  (bind _filteredoutemptyslots (CallFunction|FilterEmptySlots))
  (bind (_returnadjustedinventory _returnitemclasses) (CallFunction|FindCurrentItemClassesinInventory _filteredoutemptyslots))
  (CallFunction|SortbyItemClass _returnadjustedinventory _returnitemclasses))

(event Custom|ItemsDropped
  ;[1 1 1] Items Dropped - Drops all items
  (bind _filteredoutemptyslots (CallFunction|FilterEmptySlots))
  (CallFunction|DropItems _filteredoutemptyslots))

(event Custom|ItemDropped
  (params (SlotIndex :type Integer) (SlotInfo :type S%20Item%20Structure))
  ;[1 1 1] Item Dropped - Drops the selected item
  (CallFunction|DropItem SlotIndex SlotInfo))

(fn IncreaseAmount
  (params (ItemRef :type BP%20Base%20Item%20Object%20Reference) (SlotIndex :type Integer) (SlotInfo :type S%20Item%20Structure))
  (bind (_item _itemimage _itemname _currentamount _maximumamount _isstackable) (Utilities|Struct|BreakS_Item SlotInfo))
  (bind _iteminventorystats (Variables|/Game/Tech/Blueprints/Items/BP_BaseItem.BP_BaseItem_C|GetItemInventoryStats ItemRef))
  (bind _currentamount_2 (Utilities|Struct|BreakS_Item _iteminventorystats))
  (bind _returnvalue (+ _currentamount_2 _currentamount))
  (bind _returnvalue_2 (Math|Integer|Clamp(Integer) _returnvalue 0 _maximumamount))
  (bind _s_item (Utilities|Struct|MakeS_Item _item _itemimage _itemname _returnvalue_2 _maximumamount _isstackable))
  ;[1 1 1] Increase Amount - Adds to the current slot as much as it can an returns the remaining amount.
  (LocalVariables|SetLocalMaximumAmount _maximumamount)
  (if (<= _returnvalue _maximumamount)
    _
    (else
      (LocalVariables|SetLocalRemainingAmount (- _maximumamount _returnvalue))))
  (Utilities|Array|SetArrayElem (Variables|Default|GetInventory) SlotIndex _s_item)
  (return SlotIndex _s_item (LocalVariables|GetLocalRemainingAmount)))

(fn CheckAmount
  (params (Slot :type S%20Item%20Structure))
  (bind (_item _itemimage _itemname _currentamount _maximumamount) (Utilities|Struct|BreakS_Item Slot))
  ;[1 1 1] Check Amount - Checking if the current amount exceeds the maximum amount of the item' stack.
  (if (< _currentamount _maximumamount)
    (return true)
    (else
      (return false))))

(fn DecreaseAmount)

(fn Init
  (params (PlayerRef :type CH%20Player%20Object%20Reference) (InventoryMenu :type W%20Master%20HUD%20Object%20Reference))
  ;[1 1 1] Sets inventory size, binds event dispatchers and initiates the main inventory widget.
  (Variables|Default|SetPlayerRef PlayerRef)
  (Variables|Default|SetInventoryMenu InventoryMenu)
  (Math|Integer|DecrementInt (Variables|Default|GetNumOfSlots)
    (:%20%20
      (CallFunction|SetInventorySize)
      (EventDispatchers|BindEventtoOnItemPickUp (EventDispatchers|CreateEvent :!event Custom|ItemPickUp))
      (EventDispatchers|BindEventtoOnItemDropped (EventDispatchers|CreateEvent :!event Custom|ItemDropped))
      (EventDispatchers|BindEventtoOnItemsDropped (EventDispatchers|CreateEvent :!event Custom|ItemsDropped))
      (EventDispatchers|BindEventtoOnSortItemsbyQuantity (EventDispatchers|CreateEvent :!event Custom|SortItemsByQuantity))
      (EventDispatchers|BindEventtoOnSortItemsbyClass (EventDispatchers|CreateEvent :!event Custom|SortItemsByItemClass))
      (Default|CallOnInit (Variables|/Game/Tech/Blueprints/UI/W_MasterHUD.W_MasterHUD_C|GetW_MainInventory (Variables|Default|GetInventoryMenu)) (Variables|Default|GetNumOfSlots)))))

(fn FindEmptySlot
  ;[1 1 1] Find Empty Slot - Checks to see if a slot has a valid item class to determine if it's empty or not.
  (for (_array_element _array_index) (Variables|Default|GetInventory)
    (if (not (Utilities|IsValidClass (.Item (Utilities|Struct|BreakS_Item _array_element))))
      (return _array_index)))
  (return -1))

(fn FindStackableSlot
  (params (Item :type BP%20Base%20Item%20Class%20Reference))
  ;[1 1 1] Find Stackable Slot - Tries to find a slot which has a matching class to the passed in value.
  (for (_array_element _array_index) (Variables|Default|GetInventory)
    (if (Utilities|IsValidClass (.Item (Utilities|Struct|BreakS_Item _array_element)))
      (if (and (< (.CurrentAmount (Utilities|Struct|BreakS_Item _array_element)) (.MaximumAmount (Utilities|Struct|BreakS_Item _array_element))) (== (.Item (Utilities|Struct|BreakS_Item _array_element)) Item))
        (return _array_index _array_element))))
  (return -1 (Utilities|Struct|MakeS_Item)))

(fn AddItem
  (params (ItemClass :type BP%20Base%20Item%20Class%20Reference) (ItemRef :type BP%20Base%20Item%20Object%20Reference))
  ;[1 1 1] Add Item - Goes through the process of trying to add an item via checking if they are stackable slots or empty slots. If neither of those can be found, it will not add the item.
  (LocalVariables|SetLocalItemClass ItemClass)
  (LocalVariables|SetLocalItemRef ItemRef)
  (if (.isstackable (Variables|/Game/Tech/Blueprints/Items/BP_BaseItem.BP_BaseItem_C|GetItemInventoryStats ItemRef))
    (bind (_returnslotindex _returnslotinfo) (CallFunction|FindStackableSlot (LocalVariables|GetLocalItemClass)))
    (if (!= _returnslotindex -1)
      (bind (_returnindex _returnslotinfo_2 _remainingamount) (CallFunction|IncreaseAmount (LocalVariables|GetLocalItemRef) _returnslotindex _returnslotinfo))
      (LocalVariables|SetLocalSlotIndex _returnindex)
      (LocalVariables|SetLocalSlotInfo _returnslotinfo_2)
      (if (== _remainingamount 0)
        (return true (LocalVariables|GetLocalSlotIndex) (LocalVariables|GetLocalSlotInfo))
        (else
          (Variables|/Game/Tech/Blueprints/Items/BP_BaseItem.BP_BaseItem_C|SetItemInventoryStats (LocalVariables|GetLocalItemRef) (Utilities|Struct|MakeS_Item (.item (Variables|/Game/Tech/Blueprints/Items/BP_BaseItem.BP_BaseItem_C|GetItemInventoryStats (LocalVariables|GetLocalItemRef))) (.itemimage (Variables|/Game/Tech/Blueprints/Items/BP_BaseItem.BP_BaseItem_C|GetItemInventoryStats (LocalVariables|GetLocalItemRef))) (.itemname (Variables|/Game/Tech/Blueprints/Items/BP_BaseItem.BP_BaseItem_C|GetItemInventoryStats (LocalVariables|GetLocalItemRef))) (Math|Integer|Absolute(Integer) _remainingamount) (.maximumamount (Variables|/Game/Tech/Blueprints/Items/BP_BaseItem.BP_BaseItem_C|GetItemInventoryStats (LocalVariables|GetLocalItemRef))) (.isstackable (Variables|/Game/Tech/Blueprints/Items/BP_BaseItem.BP_BaseItem_C|GetItemInventoryStats (LocalVariables|GetLocalItemRef)))))
          (CallFunction|ItemPickUp (LocalVariables|GetLocalItemClass) (LocalVariables|GetLocalItemRef))
          (return true (LocalVariables|GetLocalSlotIndex) (LocalVariables|GetLocalSlotInfo))))
      (else
        _)))
  (bind _returnslotindex_2 (CallFunction|FindEmptySlot))
  (if (!= _returnslotindex_2 -1)
    (Utilities|Array|SetArrayElem (Variables|Default|GetInventory) _returnslotindex_2 (Utilities|Struct|MakeS_Item (.item (Variables|/Game/Tech/Blueprints/Items/BP_BaseItem.BP_BaseItem_C|GetItemInventoryStats ItemRef)) (.itemimage (Variables|/Game/Tech/Blueprints/Items/BP_BaseItem.BP_BaseItem_C|GetItemInventoryStats ItemRef)) (.itemname (Variables|/Game/Tech/Blueprints/Items/BP_BaseItem.BP_BaseItem_C|GetItemInventoryStats ItemRef)) (.currentamount (Variables|/Game/Tech/Blueprints/Items/BP_BaseItem.BP_BaseItem_C|GetItemInventoryStats ItemRef)) (.maximumamount (Variables|/Game/Tech/Blueprints/Items/BP_BaseItem.BP_BaseItem_C|GetItemInventoryStats ItemRef)) (.isstackable (Variables|/Game/Tech/Blueprints/Items/BP_BaseItem.BP_BaseItem_C|GetItemInventoryStats ItemRef))))
    (return true _returnslotindex_2 (Utilities|Struct|MakeS_Item (.item (Variables|/Game/Tech/Blueprints/Items/BP_BaseItem.BP_BaseItem_C|GetItemInventoryStats ItemRef)) (.itemimage (Variables|/Game/Tech/Blueprints/Items/BP_BaseItem.BP_BaseItem_C|GetItemInventoryStats ItemRef)) (.itemname (Variables|/Game/Tech/Blueprints/Items/BP_BaseItem.BP_BaseItem_C|GetItemInventoryStats ItemRef)) (.currentamount (Variables|/Game/Tech/Blueprints/Items/BP_BaseItem.BP_BaseItem_C|GetItemInventoryStats ItemRef)) (.maximumamount (Variables|/Game/Tech/Blueprints/Items/BP_BaseItem.BP_BaseItem_C|GetItemInventoryStats ItemRef)) (.isstackable (Variables|/Game/Tech/Blueprints/Items/BP_BaseItem.BP_BaseItem_C|GetItemInventoryStats ItemRef))))
    (else
      (return false -1 (Utilities|Struct|MakeS_Item)))))

(fn GetAmount
  (params (SlotIndex :type Integer))
  ;[1 1 1] Get Amount - Returns the current amount of an item slot
  (return (.CurrentAmount (Utilities|Struct|BreakS_Item (Utilities|Array|Get(acopy) (Variables|Default|GetInventory) SlotIndex)))))

(fn DropItem
  (params (SlotIndex :type Integer) (SlotInfo :type S%20Item%20Structure))
  ;[1 1 1] Drop Item -Given the slot, it will spawn an actor with the slot's info so that when it's picked up again, the player gets the amount dropped. Also sets the inventory's slot to be empty after spawning the item.
  (Game|SpawnActorfromClass (.Item (Utilities|Struct|BreakS_Item SlotInfo)) (Math|Transform|MakeTransform (.RandomLocation (AI|Navigation|GetRandomReachablePointinRadius (Transformation|GetWorldLocation (Variables|/Script/Engine.Character|GetCapsuleComponent (Variables|Default|GetPlayerRef))) 6e+02 0 0)) "0, 0, 0" "1,1,1") "AdjustIfPossibleButAlwaysSpawn" 0 SlotInfo 0)
  (Utilities|Array|SetArrayElem (Variables|Default|GetInventory) SlotIndex (Utilities|Struct|MakeS_Item))
  (return))

(fn DropItems
  (params (AdjustedInventory :type Array%20of%20S%20Item%20Structures))
  ;[1 1 1] Drop Items - Goes through the inventory and spawns an actor for each valid slot and applies the slot's value to the actor's item stats. It then sets the array element to be effectively an empty item struct.
  (for (_array_element _array_index) AdjustedInventory
    (Game|SpawnActorfromClass (.Item (Utilities|Struct|BreakS_Item _array_element)) (Math|Transform|MakeTransform (.RandomLocation (AI|Navigation|GetRandomReachablePointinRadius (Transformation|GetWorldLocation (Variables|/Script/Engine.Character|GetCapsuleComponent (Variables|Default|GetPlayerRef))) 6e+02 0 0)) "0, 0, 0" "1,1,1") "Undefined" 0 _array_element 0)
    (Utilities|Array|SetArrayElem (Variables|Default|GetInventory) _array_index (Utilities|Struct|MakeS_Item)))
  (return))

(fn FilterEmptySlots
  ;[1 1 1] Filter Empty Slots - Goes through the inventory and creates a new temporary inventory which only has used slots.
  (for _array_element (Variables|Default|GetInventory)
    (if (Utilities|IsValidClass (.Item (Utilities|Struct|BreakS_Item _array_element)))
      (Utilities|Array|Add (LocalVariables|GetAdjustedInventory) _array_element)))
  (return (LocalVariables|GetAdjustedInventory)))

(fn SortbyQuantity
  (params (AdjustedInventory :type Array%20of%20S%20Item%20Structures))
  ;[1 1 1] Sort By Quantity - Uses a bubble sort to rearrange the inventory from largest to smallest stack. At the end of it, empty spaces are added back to return the inventory to its original size.
  (bind _output_get (LocalVariables|SetLocalInventory AdjustedInventory))
  (LocalVariables|SetEmptySpacesToAdd (CallFunction|CalculateEmptySpacestoAdd _output_get))
  (for _index (range 0 (Utilities|Array|Length (LocalVariables|GetLocalInventory)))
    (LocalVariables|SetSwapped false)
    (bind _index_2 (Utilities|FlowControl|ForLoopwithBreak 0 (- (- (Utilities|Array|Length (LocalVariables|GetLocalInventory)) _index) 1) :!label _label)
      (:LoopBody
        (bind _output_get_2 (LocalVariables|SetI _index_2))
        (if (LocalVariables|GetSwapped)
          (goto _label Break)
          (elif (Utilities|Array|IsValidIndex (LocalVariables|GetLocalInventory) (+ _output_get_2 1))
            (LocalVariables|SetJ (+ _output_get_2 1))
            (if (< (.CurrentAmount (Utilities|Struct|BreakS_Item (Utilities|Array|Get(acopy) (LocalVariables|GetLocalInventory) (LocalVariables|GetI)))) (.CurrentAmount (Utilities|Struct|BreakS_Item (Utilities|Array|Get(acopy) (LocalVariables|GetLocalInventory) (LocalVariables|GetJ)))))
              (Utilities|Array|Swap (LocalVariables|GetLocalInventory) (LocalVariables|GetI) (LocalVariables|GetJ))
              (LocalVariables|SetSwapped true)))))))
  (for _index_3 (range 0 (LocalVariables|GetEmptySpacesToAdd))
    (Utilities|Array|Add (LocalVariables|GetLocalInventory) (Utilities|Struct|MakeS_Item)))
  (Variables|Default|SetInventory (LocalVariables|GetLocalInventory))
  (return))

(fn SetInventorySize
  ;[1 1 1] Set Inventory Size - Sets the size of the inventory
  (for _index (range 0 (Variables|Default|GetNumOfSlots))
    (Utilities|Array|Add (Variables|Default|GetInventory) (Utilities|Struct|MakeS_Item)))
  (return))

(fn FindCurrentItemClassesinInventory
  (params (AdjustedInventory :type Array%20of%20S%20Item%20Structures))
  ;[1 1 1] Find Current Item Classes in Inventory - Finds all unqiue item classes included in the inventory.
  (for _array_element AdjustedInventory
    (if (not (Utilities|Array|ContainsItem (LocalVariables|GetItemClasses) (.Item (Utilities|Struct|BreakS_Item _array_element))))
      (Utilities|Array|AddUnique (LocalVariables|GetItemClasses) (.Item (Utilities|Struct|BreakS_Item _array_element)))))
  (return AdjustedInventory (LocalVariables|GetItemClasses)))

(fn SortbyItemClass
  (params (AdjustedInventory :type Array%20of%20S%20Item%20Structures) (ItemClasses :type Array%20of%20BP%20Base%20Item%20Class%20References))
  ;[1 1 1] Sort By Item Class - Rearranges the inventory based on the item class order in the item classes array.
  (LocalVariables|SetLocalInventory AdjustedInventory)
  (LocalVariables|SetLocalItemClassesRef ItemClasses)
  (if (!= 0 (Utilities|Array|Length (LocalVariables|GetLocalItemClassesRef)))
    (for (_array_element _array_index) (LocalVariables|GetLocalInventory)
      (LocalVariables|SetArrayIndex _array_index)
      (if (== (.Item (Utilities|Struct|BreakS_Item _array_element)) (Utilities|Array|Get(acopy) (LocalVariables|GetLocalItemClassesRef)))
        (bind (_array_element_2 _array_index_2) (Utilities|Array|ForEachLoopwithBreak (LocalVariables|GetLocalInventory) :!label _label)
          (:LoopBody
            (if (!= (.Item (Utilities|Struct|BreakS_Item _array_element_2)) (Utilities|Array|Get(acopy) (LocalVariables|GetLocalItemClassesRef)))
              (Utilities|Array|Swap (LocalVariables|GetLocalInventory) _array_index_2 (LocalVariables|GetArrayIndex))
              (goto _label Break))))))
    (bind _returnvalue (Utilities|Array|RemoveItem (LocalVariables|GetLocalItemClassesRef) (Utilities|Array|Get(acopy) (LocalVariables|GetLocalItemClassesRef))))
    (if _returnvalue
      (CallFunction|SortbyItemClass (LocalVariables|GetLocalInventory) (LocalVariables|GetLocalItemClassesRef))
      (return))
    (else
      (for _index (range 0 (CallFunction|CalculateEmptySpacestoAdd (LocalVariables|GetLocalInventory)))
        (Utilities|Array|Add (LocalVariables|GetLocalInventory) (Utilities|Struct|MakeS_Item)))
      (Variables|Default|SetInventory (LocalVariables|GetLocalInventory))
      (return))))

(fn CalculateEmptySpacestoAdd
  (params (AdjustedInventory :type Array%20of%20S%20Item%20Structures))
  ;[1 1 1] Calculate Empty Spaces to Add - Subtracts the length of the adjusted inventory from the original to determine the number of spaces remove and therefore to add.
  (Variables|Default|SetLocalInventory AdjustedInventory)
  (bind _output_get (LocalVariables|SetEmptySpacesToAdd (- (Utilities|Array|Length (Variables|Default|GetInventory)) (Utilities|Array|Length (Variables|Default|GetLocalInventory)))))
  (return _output_get))