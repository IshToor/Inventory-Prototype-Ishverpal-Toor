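; Player controller that bootstraps the player character and master HUD and routes player input.
; On BeginPlay it finds the CH_Player actor in the level, creates the HUD widget with that reference, then links itself to the character and initializes it.
; Movement, look, jump and interact inputs forward to the character.
; The inventory input toggles the HUD's inventory, updates cursor visibility and sets Game and UI input mode focused on it.
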(event Custom|ToggleMouseCursor
  ;[1 1 1] Toggle Mouse Cursor
  (Variables|Default|SetbShowMouseCursor (not (Variables|Default|GetMouseVisibility)))
  (Input|SetInputModeGameandUI self (Variables|/Game/Tech/Blueprints/UI/W_MasterHUD.W_MasterHUD_C|GetW_MainInventory (Variables|Default|GetMasterHUD)) "DoNotLock" false))

(event EventBeginPlay
  ;[1 1 1] Initialisation - Finds player, creates HUD & initialise the player
  (bind _returnvalue (Actor|GetActorOfClass "/Game/Tech/Blueprints/Characters/CH_Player.CH_Player_C"))
  (bind _output_get (Variables|Default|SetPlayerCharacterRef _returnvalue))
  (bind _returnvalue_2 (UserInterface|CreateWidget "/Game/Tech/Blueprints/UI/W_MasterHUD.W_MasterHUD_C" self _output_get))
  (bind _output_get_2 (Variables|Default|SetMasterHUD _returnvalue_2))
  (UserInterface|Viewport|AddtoViewport _output_get_2 0)
  (Variables|/Game/Tech/Blueprints/Characters/CH_Player.CH_Player_C|SetPlayerControllerRef (Variables|Default|GetPlayerCharacterRef) self)
  (Default|Init (Variables|Default|GetPlayerCharacterRef)))

(event Input|ActionEvents|InputActionInteract
  (params (Key :type Key%20Structure :default "None"))
  ;[1 1 1] Controls
  (:Pressed
    (Default|Interact (Variables|Default|GetPlayerCharacterRef))))

(event Input|ActionEvents|InputActionOpen/CloseInventory
  (params (Key :type Key%20Structure :default "None"))
  ;[1 1 1] Controls
  (:Pressed
    (Default|CallOnToggleVisibility (Variables|/Game/Tech/Blueprints/UI/W_MasterHUD.W_MasterHUD_C|GetW_MainInventory (Variables|Default|GetMasterHUD)))
    (CallFunction|ToggleMouseCursor)))

(event Input|ActionEvents|InputActionJump
  (params (Key :type Key%20Structure :default "None"))
  (bind _playercharacterref (Variables|Default|GetPlayerCharacterRef))
  ;[1 1 1] Controls
  (:Pressed
    (Default|OnJump _playercharacterref))
  (:Released
    (Default|OnStopJump _playercharacterref)))

(event Input|AxisEvents|InputAxisLookUp
  (params (AxisValue :type Float%20%28single-precision%29))
  ;[1 1 1] Controls
  (Default|OnLookUp (Variables|Default|GetPlayerCharacterRef) AxisValue))

(event Input|AxisEvents|InputAxisTurn
  (params (AxisValue :type Float%20%28single-precision%29))
  ;[1 1 1] Controls
  (Default|OnTurn (Variables|Default|GetPlayerCharacterRef) AxisValue))

(event Input|AxisEvents|InputAxisMoveForward
  (params (AxisValue :type Float%20%28single-precision%29))
  ;[1 1 1] Controls
  (Default|OnMoveForward (Variables|Default|GetPlayerCharacterRef) AxisValue))

(event Input|AxisEvents|InputAxisMoveRight
  (params (AxisValue :type Float%20%28single-precision%29))
  ;[1 1 1] Controls
  (Default|OnMoveRight (Variables|Default|GetPlayerCharacterRef) AxisValue))

(fn ConstructionScript)